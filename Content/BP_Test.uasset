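; BP_Test is a scratch actor for trying out serialization.
; On BeginPlay it writes a string with a SerializerObject, feeds the bytes into a DeSerializerObject and prints the string it reads back.
; Disconnected chains round-trip a BP_object_test through byte serialization, including a compressed file at a hardcoded disk path.
; Other unwired nodes poke at EasySettingsSubsystem quality, resolution and container values.
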(event `self.ReceiveBeginPlay`
  (bind _returnvalue (`|GenericCreateObject` "/Script/DataSerializer.SerializerObject"))
  (`SerializerObject.Prepare` _returnvalue)
  (`SerializerObject.SerializeString` _returnvalue "fjjftjfjt")
  (bind _outbytes (`SerializerObject.GetBytes` _returnvalue))
  (bind _returnvalue_2 (`|GenericCreateObject` "/Script/DataSerializer.DeSerializerObject"))
  (`DeSerializerObject.Start` _returnvalue_2 _outbytes)
  (bind _outstring (`DeSerializerObject.TryReadString` _returnvalue_2))
  (`KismetSystemLibrary.PrintString` _outstring))

(fn `UserConstructionScript`)